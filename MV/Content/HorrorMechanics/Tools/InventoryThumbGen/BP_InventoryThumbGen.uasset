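; Editor tool actor that renders a static mesh, skeletal mesh or child actor into an inventory thumbnail texture.
; The construction script positions the item, aims the scene capture at it and refreshes an optional preview mesh.
; Separate color and HDR alpha captures at scaled resolution are merged by M_InvertAlpha into a thumbnail-sized target.
; RenderTexture saves that target as an editor-only static UI texture.
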(event `RenderTextureEv`
  (params (CreateTexture :type Boolean))
  (bind _fixedrendertarget (`self.FixedRenderTarget`))
  (bind _invertalphamat (`self.InvertAlphaMat`))
  (bind _scenecapturecomponent2d (`self.SceneCaptureComponent2D`))
  (bind _scenecapturecomponent2d_2 (`self.SceneCaptureComponent2D`))
  (bind _thumbnailresolution (`self.ThumbnailResolution`))
  (bind _skeletalmeshcomponent (`self.SkeletalMeshComponent`))
  (bind _childactor (`ChildActorComponent.ChildActor` (`self.ChildActorComponent`)))
  (bind _returnvalue (`KismetMathLibrary.FTrunc` (* (`self.ThumbnailResolution`) (`self.RenderScale`))))
  ;[0.2 0.2 0.2 0.2] Render
  (`|ExecutionSequence`
    (:`then_0`
      (`/Engine/EditorBlueprintResources/StandardMacros.IsValid` (`self.ColorRenderTarget`)
        (:`Is Not Valid`
          (bind _returnvalue_2 (`KismetRenderingLibrary.CreateRenderTarget2D` _returnvalue _returnvalue))
          (set `self.ColorRenderTarget` _returnvalue_2)
          (`/Engine/EditorBlueprintResources/StandardMacros.IsValid` (`self.FixedRenderTarget`)
            (:`Is Not Valid`
              (bind _returnvalue_3 (`KismetRenderingLibrary.CreateRenderTarget2D` _thumbnailresolution _thumbnailresolution))
              (set `self.FixedRenderTarget` _returnvalue_3))))))
    (:`then_1`
      (`/Engine/EditorBlueprintResources/StandardMacros.IsValid` (`self.AlphaRenderTarget`)
        (:`Is Not Valid`
          (bind _returnvalue_4 (`KismetRenderingLibrary.CreateRenderTarget2D` _returnvalue _returnvalue))
          (set `self.AlphaRenderTarget` _returnvalue_4))))
    (:`then_2`
      (`/Engine/EditorBlueprintResources/StandardMacros.IsValid` _childactor
        (:`Is Valid`
          (`SceneCaptureComponent.ShowOnlyActorComponents` _scenecapturecomponent2d _childactor))
        (:`Is Not Valid`
          (`/Engine/EditorBlueprintResources/StandardMacros.IsValid` (`SkinnedMeshComponent.SkeletalMesh` _skeletalmeshcomponent)
            (:`Is Valid`
              (`SceneCaptureComponent.ShowOnlyComponent` _scenecapturecomponent2d _skeletalmeshcomponent))
            (:`Is Not Valid`
              (`SceneCaptureComponent.ShowOnlyComponent` _scenecapturecomponent2d (`self.StaticMeshComponent`)))))))
    (:`then_3`
      (set `SceneCaptureComponent2D.CaptureSource` "SCS_FinalColorLDR" _scenecapturecomponent2d_2)
      (set `SceneCaptureComponent2D.TextureTarget` (`self.ColorRenderTarget`) _scenecapturecomponent2d_2)
      (`SceneCaptureComponent2D.CaptureScene` _scenecapturecomponent2d_2)
      (set `SceneCaptureComponent2D.CaptureSource` "SCS_SceneColorHDR" _scenecapturecomponent2d_2)
      (set `SceneCaptureComponent2D.TextureTarget` (`self.AlphaRenderTarget`) _scenecapturecomponent2d_2)
      (`SceneCaptureComponent2D.CaptureScene` _scenecapturecomponent2d_2))
    (:`then_4`
      (`/Engine/EditorBlueprintResources/StandardMacros.IsValid` (`self.InvertAlphaMat`)
        (:`Is Not Valid`
          (bind _returnvalue_5 (`KismetMaterialLibrary.CreateDynamicMaterialInstance` "/Game/HorrorMechanics/Tools/InventoryThumbGen/Materials/M_InvertAlpha.M_InvertAlpha"))
          (set `self.InvertAlphaMat` _returnvalue_5))))
    (:`then_5`
      (`MaterialInstanceDynamic.SetTextureParameterValue` _invertalphamat "Color" (`self.ColorRenderTarget`))
      (`MaterialInstanceDynamic.SetTextureParameterValue` _invertalphamat "Alpha" (`self.AlphaRenderTarget`))
      (`MaterialInstanceDynamic.SetScalarParameterValue` _invertalphamat "Exp" (`self.Gamma`)))
    (:`then_6`
      (`/Engine/EditorBlueprintResources/StandardMacros.IsValid` _fixedrendertarget
        (:`Is Valid`
          (`KismetRenderingLibrary.ClearRenderTarget2D` _fixedrendertarget)
          (set `TextureRenderTarget.TargetGamma` 2.2 _fixedrendertarget)
          (`KismetRenderingLibrary.DrawMaterialToRenderTarget` _fixedrendertarget (`self.InvertAlphaMat`))
          (if CreateTexture
            (bind _returnvalue_6 (`KismetRenderingLibrary.RenderTargetCreateStaticTexture2DEditorOnly` _fixedrendertarget (`KismetStringLibrary.Concat_StrStr` (`self.Directory`) "/" (`self.TextureName`)) "TC_EditorIcon"))
            (set `Texture.LODGroup` "TEXTUREGROUP_UI" _returnvalue_6)
            (set `Texture.CompressionSettings` "TC_EditorIcon" _returnvalue_6)))))))

(event `UpdateMesh`
  (bind _scenecapturecomponent2d (`self.SceneCaptureComponent2D`))
  ;[0.2 0.2 0.2 0.2] Update
  (`|ExecutionSequence`
    (:`then_0`
      (`SceneComponent.K2_SetRelativeTransform` (`self.Items`) (`self.ItemTransform`) false false)
      (`StaticMeshComponent.SetStaticMesh` (`self.StaticMeshComponent`) (`self.StaticMesh`))
      (`ChildActorComponent.SetChildActorClass` (`self.ChildActorComponent`) (`self.ActorClass`))
      (`SkinnedMeshComponent.SetSkinnedAssetAndUpdate` (`self.SkeletalMeshComponent`) (`self.SkeletalMesh`) true))
    (:`then_1`
      (`SceneComponent.K2_SetRelativeLocation` _scenecapturecomponent2d (`self.CameraLocation`) false false)
      (`SceneComponent.K2_SetWorldRotation` _scenecapturecomponent2d (`KismetMathLibrary.FindLookAtRotation` (`SceneComponent.K2_GetComponentLocation` _scenecapturecomponent2d) (`SceneComponent.K2_GetComponentLocation` (`self.Items`))) false false)
      (`CameraComponent.SetFieldOfView` (`self.PreviewCamera`) (`SceneCaptureComponent2D.FOVAngle` _scenecapturecomponent2d)))))

(event `UpdatePreview`
  (bind _previewmat (`self.PreviewMat`))
  (`SceneComponent.K2_SetRelativeTransform` (`self.PreviewMesh`) (`KismetMathLibrary.MakeTransform` (0.0 0.0 200.0) (`KismetMathLibrary.ComposeRotators` (struct :`Yaw` 90.0 :`Roll` 90.0) (`KismetMathLibrary.NegateRotator` (`self.K2_GetActorRotation`)))) false false)
  (`self.RenderTextureEv` false)
  (`/Engine/EditorBlueprintResources/StandardMacros.IsValid` (`self.PreviewMat`)
    (:`Is Valid`
      _)
    (:`Is Not Valid`
      (bind _returnvalue (`KismetMaterialLibrary.CreateDynamicMaterialInstance` "/Game/HorrorMechanics/Tools/InventoryThumbGen/Materials/M_ThumbnailPreview.M_ThumbnailPreview"))
      (set `self.PreviewMat` _returnvalue)
      (`PrimitiveComponent.SetMaterial` (`self.PreviewMesh`) 0 (`self.PreviewMat`))))
  (`/Engine/EditorBlueprintResources/StandardMacros.IsValid` _previewmat
    (:`Is Valid`
      (`/Engine/EditorBlueprintResources/StandardMacros.IsValid` (`self.FixedRenderTarget`)
        (:`Is Valid`
          (`MaterialInstanceDynamic.SetTextureParameterValue` _previewmat "BaseTexture" (`self.FixedRenderTarget`))
          (`MaterialInstanceDynamic.SetScalarParameterValue` _previewmat "Alpha" 1.0)
          (`MaterialInstanceDynamic.SetScalarParameterValue` _previewmat "Emissive" 1.0)
          (`SceneComponent.SetVisibility` (`self.PreviewMesh`) (`self.ShowResult`) false))))))

(fn `RenderTexture`
  (`self.RenderTextureEv` true))

(fn `UserConstructionScript`
  (`self.UpdateMesh`)
  (`self.UpdatePreview`))