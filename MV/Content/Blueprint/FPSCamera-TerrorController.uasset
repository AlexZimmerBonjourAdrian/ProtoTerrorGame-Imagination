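; First-person player character Blueprint, named for a terror game, with walking, mouse look, jumping and a toggleable flashlight.
; Movement axes push along the camera's forward and right vectors, each multiplied by ForwardAxis, while Mouse2D drives controller yaw and inverted-Y pitch.
; The F key flip-flops flashlight visibility, hiding it on the first press.
; The Dash function is an empty stub, and Tick does nothing.
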(event `self.ReceiveTick`
  (params (DeltaSeconds :type "Float (single-precision)")))

(event `InputAxis|Movement_X`
  (params (AxisValue :type "Float (single-precision)"))
  (bind _output_get (set `self.Axis Value` AxisValue))
  (`self.AddMovementInput` (* (`SceneComponent.GetForwardVector` (`self.Camera`)) (`self.ForwardAxis`)) _output_get))

(event `InputAxis|Movement_Y`
  (params (AxisValue :type "Float (single-precision)"))
  (bind _output_get (set `self.Axis Value` AxisValue))
  (`self.AddMovementInput` (* (`SceneComponent.GetRightVector` (`self.Camera`)) (`self.ForwardAxis`)) _output_get))

(event `InputVectorAxis|Mouse2D`
  (params (AxisValue :type "Vector Structure"))
  (`self.AddControllerYawInput` (.x AxisValue))
  (`self.AddControllerPitchInput` (* (.y AxisValue) -1.0)))

(event `Key|F`
  (params (Key :type "Key Structure"))
  (:`Pressed`
    (`/Engine/EditorBlueprintResources/StandardMacros.FlipFlop`
      (:`A`
        (`SceneComponent.SetVisibility` (`self.FlashLight`) false false))
      (:`B`
        (`SceneComponent.SetVisibility` (`self.FlashLight`) true false)))))

(event `InputAction|Jump_Trigger`
  (params (Key :type "Key Structure"))
  (:`Pressed`
    (`self.Jump`)))

(fn `Dash`
  (params (AxisValue :type "Float (double-precision)")))

(fn `UserConstructionScript`)