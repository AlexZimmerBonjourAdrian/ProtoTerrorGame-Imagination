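; First-person character Blueprint handling camera-relative movement, mouse look, jump and a directional dash.
; Both movement axis events overwrite a shared IsForward flag and AxisValue, which Dash reads to pick the camera's forward or right vector and its sign.
; Each dash launches the character twice, separated by a cooldown delay, with a DoOnce reset after a second delay.
; Tick and DashRight print debug text, and the Dash function is an empty stub.
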(event `self.ReceiveTick`
  (params (DeltaSeconds :type "Float (single-precision)"))
  (`KismetSystemLibrary.PrintString` (`KismetStringLibrary.Conv_BoolToString` (`self.IsForward`))))

(event `InputAxis|Movement_X`
  (params (AxisValue :type "Float (single-precision)"))
  (set `self.IsForward` true)
  (bind _output_get (set `self.Axis Value` AxisValue))
  (`self.AddMovementInput` (* (`SceneComponent.GetForwardVector` (`self.Camera`)) (`self.ForwardAxis`)) _output_get))

(event `InputAxis|Movement_Y`
  (params (AxisValue :type "Float (single-precision)"))
  (set `self.IsForward` false)
  (bind _output_get (set `self.Axis Value` AxisValue))
  (`self.AddMovementInput` (* (`SceneComponent.GetRightVector` (`self.Camera`)) (`self.ForwardAxis`)) _output_get))

(event `InputVectorAxis|Mouse2D`
  (params (AxisValue :type "Vector Structure"))
  (`self.AddControllerYawInput` (.x AxisValue))
  (`self.AddControllerPitchInput` (* (.y AxisValue) -1.0)))

(event `InputAction|Dash`
  (params (Key :type "Key Structure"))
  (:`Pressed`
    (if (`self.IsForward`)
      (`self.DashForward`)
      (else
        (`self.DashRight`)))))

(event `DashForward`
  (bind _returnvalue (* (* (`SceneComponent.GetForwardVector` (`self.Camera`)) (`self.DashMultiply`)) (`self.Axis Value`)))
  (`/Engine/EditorBlueprintResources/StandardMacros.DoOnce` false :!label _label
    (:`Completed`
      (`self.LaunchCharacter` _returnvalue)
      (`KismetSystemLibrary.Delay` (`self.Coultdown Dash`))
      (`self.LaunchCharacter` _returnvalue)
      (`KismetSystemLibrary.Delay` (`self.Coultdown Dash`))
      (goto _label :!via `Reset`))))

(event `InputAction|Jump_Trigger`
  (params (Key :type "Key Structure"))
  (:`Pressed`
    (`self.Jump`)))

(event `DashRight`
  (bind _returnvalue (* (* (`SceneComponent.GetRightVector` (`self.Camera`)) (`self.DashMultiply`)) (`self.Axis Value`)))
  (`KismetSystemLibrary.PrintString` "EntraEnRigjtDash")
  (`/Engine/EditorBlueprintResources/StandardMacros.DoOnce` false :!label _label_2
    (:`Completed`
      (`self.LaunchCharacter` _returnvalue)
      (`KismetSystemLibrary.Delay` (`self.Coultdown Dash`))
      (`self.LaunchCharacter` _returnvalue)
      (`KismetSystemLibrary.Delay` (`self.Coultdown Dash`))
      (goto _label_2 :!via `Reset`))))

(fn `Dash`
  (params (AxisValue :type "Float (double-precision)")))

(fn `UserConstructionScript`)